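; Blueprint function library of debug helpers for visualizing Myo orientation, EMG and vector data.
; DrawOrientation draws a short-lived forward arrow tipped with a rotated box, and DrawVectorArrow draws any scaled vector.
; PrintMyoEmg prints the EMG streams separated by commas, including a trailing one because the last-index check compares against Length.
; DrawMyoEmgArrows renders streams as a row of arrows along Y, with value-scaled lengths rotated by Orientation.
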(fn DrawOrientation
  (params (Orientation :type Rotator :default "0, 0, 0") (Color :type Linear%20Color%20Structure) (Origin :type Vector :default "0, 0, 0"))
  (bind _returnvalue (Math|Vector|GetForwardVector Orientation))
  (bind _returnvalue_2 (* _returnvalue 5e+02))
  (bind _returnvalue_3 (+ Origin _returnvalue_2))
  (Rendering|Debug|DrawDebugArrow 0 Origin _returnvalue_3 2e+02 Color 0.04)
  (Rendering|Debug|DrawDebugBox 0 _returnvalue_3 "50.000000,50.000000,50.000000" Color Orientation 0.04))

(fn PrintMyoEmg
  (params (data :type Myo%20Emg%20Data%20Structure))
  (bind _streams (Utilities|Struct|BreakMyoEmgData data))
  (LocalVariables|SetPrintString "")
  (for (_array_element _array_index) _streams
    (Math|Integer|CompareInt _array_index (Utilities|Array|Length _streams)
      (:==
        (LocalVariables|SetPrintString (Utilities|String|Append (LocalVariables|GetPrintString) (Utilities|String|ToString(Integer) _array_element))) ; final no comma
      )
      (:<
        (LocalVariables|SetPrintString (Utilities|String|Append (Utilities|String|Append (LocalVariables|GetPrintString) (Utilities|String|ToString(Integer) _array_element)) ", ")) ; all other comma
      )))
  (Development|PrintString 0 (LocalVariables|GetPrintString)))

(fn DrawMyoEmgArrows
  (params (data :type Myo%20Emg%20Data%20Structure) (Origin :type Vector) (Offset :type Vector) (HeightScale :type Float%20%28single-precision%29) (SeparationScale :type Float%20%28single-precision%29) (Orientation :type Rotator :default "0, 0, 0"))
  (for (_array_element _array_index) (Utilities|Struct|BreakMyoEmgData data)
    (Rendering|Debug|DrawDebugArrow :LineStart (+ Origin (+ Offset (Math|Vector|MakeVector 0.0 (* _array_index (* SeparationScale 3e+01)) 0.0))) :LineEnd (+ (+ Origin (+ Offset (Math|Vector|MakeVector 0.0 (* _array_index (* SeparationScale 3e+01)) 0.0))) (Math|Vector|RotateVector (Math|Vector|MakeVector 0.0 0.0 (* HeightScale (Math|Conversions|ToFloat(Integer) _array_element))) Orientation)) :ArrowSize 2e+01)))

(fn DrawVectorArrow
  (params (Vector :type Vector :default "0, 0, 0") (Origin :type Vector :default "0, 0, 0") (Scale :type Float%20%28single-precision%29) (Color :type Linear%20Color%20Structure))
  (Rendering|Debug|DrawDebugArrow 0 Origin (+ Origin (* Vector Scale)) 1.0 Color 0.0))